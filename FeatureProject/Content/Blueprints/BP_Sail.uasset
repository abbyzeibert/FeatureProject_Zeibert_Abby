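; Player-controlled sail actor that the player steers to match a randomly shifting wind direction.
; Enhanced Input steers the sail and toggles sail and mast, which animate through timelines for sail scale and mast pitch.
; While the sail is out, Tick applies steering plus drift unless locked, then stores its offset from the wind in SailMatch.
; A looping delay re-rolls the wind, and yaw eases toward the sail position each frame.
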(event Custom|ToggleMast
  (if (Variables|Default|GetIsMastUp)
    (CallFunction|ToggleSail)
    (bind _mastangle (Timeline|MastMovement Play)
      (:Update
        (Transformation|SetActorRotation (Math|Rotator|MakeRotator 0.0 _mastangle 0.0)))
      (:ChangeState
        (if (Variables|Default|GetIsMastUp)
          (Variables|Default|SetIsMastUp false)
          (else
            (Variables|Default|SetIsMastUp true)))))
    (else
      (Timeline|MastMovement Reverse))))

(event Custom|Toggle%20Sail
  (if (Variables|Default|GetIsMastUp)
    (if (Variables|Default|GetIsSailOut)
      (Variables|Default|SetSailPos 0.0)
      (bind _sailscale (Timeline|SailMovement Play)
        (:Update
          (Development|PrintString (Utilities|String|ToString(Float) _sailscale))
          (Transformation|SetRelativeScale3D (Variables|Default|GetSailPivot) (Math|Vector|MakeVector _sailscale 1.0 1.0)))
        (:Finished
          (Development|PrintString "finished"))
        (:SailActive
          (if (Variables|Default|GetIsSailOut)
            (Variables|Default|SetIsSailOut false)
            (else
              (Variables|Default|SetIsSailOut true)))))
      (else
        (Timeline|SailMovement Reverse)))
    (else
      (Development|PrintString "didnt run"))))

(event Input|EnhancedActionEvents|EnhancedInputActionIA_Move
  (params (ActionValue :type Float%20%28double-precision%29) (ElapsedSeconds :type Float%20%28double-precision%29) (TriggeredSeconds :type Float%20%28double-precision%29) (InputAction :type Input%20Action%20Object%20Reference :default "/Game/Blueprints/GameSystems/IA_Move.IA_Move"))
  (:Triggered
    (Variables|Default|SetTurnDir ActionValue))
  (:Completed
    (Variables|Default|SetTurnDir 0.0)))

(event Input|EnhancedActionEvents|EnhancedInputActionIA_Sail
  (params (ActionValue :type Boolean) (ElapsedSeconds :type Float%20%28double-precision%29) (TriggeredSeconds :type Float%20%28double-precision%29) (InputAction :type Input%20Action%20Object%20Reference :default "/Game/Blueprints/GameSystems/IA_Sail.IA_Sail"))
  (CallFunction|ToggleSail))

(event Input|EnhancedActionEvents|EnhancedInputActionIA_Mast
  (params (ActionValue :type Boolean) (ElapsedSeconds :type Float%20%28double-precision%29) (TriggeredSeconds :type Float%20%28double-precision%29) (InputAction :type Input%20Action%20Object%20Reference :default "/Game/Blueprints/GameSystems/IA_Mast.IA_Mast"))
  (CallFunction|ToggleMast))

(event EventBeginPlay
  (Utilities|FlowControl|Sequence
    (:then_0
      (bind _asbp_player_controller (Utilities|Casting|CastToBP_PlayerController (Game|GetPlayerController 0)))
      (bind _output_get (Variables|Default|SetPlayerController _asbp_player_controller))
      (Utilities|IsValid (PlayerController|LocalPlayerSubsystems|GetEnhancedInputLocalPlayerSubsystem _output_get)
        (:Is%20Valid
          (Input|AddMappingContext (PlayerController|LocalPlayerSubsystems|GetEnhancedInputLocalPlayerSubsystem _output_get) "/Game/Blueprints/GameSystems/IMC_Controls.IMC_Controls" 0 "(bIgnoreAllPressedKeysUntilRelease=True,bForceImmediately=False,bNotifyUserSettings=False)"))))
    (:then_1
      (Utilities|FlowControl|Delay (Math|Random|RandomFloatinRange 5.0 1e+01) :!label _label)
      (CallFunction|SetWindPos)
      (goto _label))))

(event Collision|EventActorBeginOverlap
  (params (OtherActor :type Actor%20Object%20Reference)))

(event EventTick
  (params (DeltaSeconds :type Float%20%28single-precision%29))
  (if (Variables|Default|GetIsSailOut)
    (bind _output_get (Variables|Default|SetSailPos (Math|Float|Clamp(Float) (+ (* (Variables|Default|GetTurnDir) (Variables|Default|GetTurnSpeed) DeltaSeconds) (Variables|Default|GetSailPos)) 0.01 1.8e+02)))
    (if (Variables|Default|GetLocked)
      _
      (else
        (Variables|Default|SetSailPos (+ (Variables|Default|GetSailPos) (* (Variables|Default|GetDriftSpeed) DeltaSeconds)))))
    (CallFunction|ChangeSailAngle _output_get)
    (Variables|Default|SetSailMatch (Math|Float|Absolute(Float) (- (Variables|Default|GetSailPos) (Variables|Default|GetWindPos))))
    (else
      (CallFunction|ChangeSailAngle (Variables|Default|GetSailPos)))))

(fn ConstructionScript)

(fn SetWindPos
  (Variables|Default|SetWindPos (Math|Random|RandomFloatinRange 1.0 1.8e+02)))

(fn ChangeSailAngle
  (params (TurnTo :type Float%20%28double-precision%29))
  (bind _returnvalue (Transformation|GetActorRotation))
  (bind _output_get (LocalVariables|SetCurAngle (Math|Interpolation|Ease "SinusoidalInOut" 0.5 (.yaw _returnvalue) TurnTo)))
  (Transformation|SetActorRotation (Math|Rotator|MakeRotator (.roll _returnvalue) (.pitch _returnvalue) _output_get)))